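; BP_God is the actor that drops obstacles into three lanes, paid for with Badluck from GM_Main.
; On BeginPlay it selects the 100t obstacle by default and registers itself as God on the game mode.
; SetCurrentObject switches between 100t, Piano and Animal, and SpawnObstacle spawns that class at the chosen lane's SpawnBox.
; The cost is read from the spawned actor, which is destroyed if unaffordable, otherwise its BadluckCost is deducted.
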(event EventBeginPlay
  (Variables|Default|SetcurrentObject "/Game/BP/FallingObjects/100t.100t_C")
  (bind _asgm_main (Utilities|Casting|CastToGM_Main (Game|GetGameMode)))
  (Variables|/Game/BP/GM_Main.GM_Main_C|SetGod _asgm_main self))

(fn ConstructionScript)

(fn SpawnObstacle
  (params (laneNumber :type Integer))
  (bind _newparam (CallFunction|GetLaneTransform laneNumber))
  (bind _returnvalue (Game|SpawnActorfromClass (Variables|Default|GetcurrentObject) _newparam "Undefined" 0 0))
  (bind _asgm_main (Utilities|Casting|CastToGM_Main (Game|GetGameMode)))
  (if (> (Variables|/Game/BP/FallingObjects/FallingObject.FallingObject_C|GetBadluckCost _returnvalue) (Variables|/Game/BP/GM_Main.GM_Main_C|GetBadluck _asgm_main))
    (Actor|DestroyActor _returnvalue)
    (else
      (Default|AddBadluck _asgm_main (* (Variables|/Game/BP/FallingObjects/FallingObject.FallingObject_C|GetBadluckCost _returnvalue) -1.0)))))

(fn GetLaneTransform
  (params (laneNumber :type Integer))
  (switch int laneNumber
    (:1
      (return (Transformation|GetWorldTransform (Variables|Default|GetSpawnBox1))))
    (:2
      (return (Transformation|GetWorldTransform (Variables|Default|GetSpawnBox2))))
    (:3
      (return (Transformation|GetWorldTransform (Variables|Default|GetSpawnBox3))))))

(fn SetCurrentObject
  (params (ObjectNumber :type Integer))
  (switch int ObjectNumber
    (:1
      (Variables|Default|SetcurrentObject "/Game/BP/FallingObjects/100t.100t_C"))
    (:2
      (Variables|Default|SetcurrentObject "/Game/BP/FallingObjects/Piano.Piano_C"))
    (:3
      (Variables|Default|SetcurrentObject "/Game/BP/FallingObjects/Animal.Animal_C"))))