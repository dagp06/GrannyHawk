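; BP_PlayZone is a play area actor that follows the player along the world X axis and registers itself with GM_Main on BeginPlay.
; Each tick it snaps its root to the X of the player's mesh, keeping its own Y and Z.
; It also moves BPGod along X to the player's position offset by X velocity times GodSpawnDistance, so the God leads in the direction of travel.
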(event EventBeginPlay
  (bind _asgm_main (Utilities|Casting|CastToGM_Main (Game|GetGameMode)))
  (Variables|/Game/BP/GM_Main.GM_Main_C|SetPlayZone _asgm_main self))

(event EventTick
  (params (DeltaSeconds :type Float%20%28single-precision%29))
  (CallFunction|UpdatePosition)
  (CallFunction|AjustGodPosition))

(fn ConstructionScript)

(fn UpdatePosition
  (bind _defaultsceneroot (Variables|Default|GetDefaultSceneRoot))
  (bind _returnvalue (Transformation|GetWorldLocation _defaultsceneroot))
  (bind _asgm_main (Utilities|Casting|CastToGM_Main (Game|GetGameMode))
    (:then
      (if (Utilities|IsValid (Variables|/Game/BP/GM_Main.GM_Main_C|GetPlayer _asgm_main))
        (Transformation|SetWorldLocation (Variables|Default|GetDefaultSceneRoot) (Math|Vector|MakeVector (.x (.location (Transformation|GetWorldTransform (Variables|/Script/Engine.DefaultPawn|GetMeshComponent (Variables|/Game/BP/GM_Main.GM_Main_C|GetPlayer _asgm_main))))) (.y _returnvalue) (.z _returnvalue)) false false)))
    (:CastFailed
      _))
  (return))

(fn AjustGodPosition
  (bind _bp_god (Variables|Default|GetBP_God))
  (bind _returnvalue (Transformation|GetWorldLocation _bp_god))
  (bind _asgm_main (Utilities|Casting|CastToGM_Main (Game|GetGameMode)))
  (Transformation|SetWorldLocation (Variables|Default|GetBP_God) (Math|Vector|MakeVector (+ (.x (Transformation|GetWorldLocation (Variables|/Game/ThirdPersonBP/Blueprints/SkaterDefaultPawn.SkaterDefaultPawn_C|GetSkeletalMesh (Variables|/Game/BP/GM_Main.GM_Main_C|GetPlayer _asgm_main)))) (* (.x (Variables|/Script/Engine.MovementComponent|GetVelocity (Variables|/Game/ThirdPersonBP/Blueprints/SkaterDefaultPawn.SkaterDefaultPawn_C|GetFloatingPawnMovement (Variables|/Game/BP/GM_Main.GM_Main_C|GetPlayer _asgm_main)))) (Variables|Default|GetGodSpawnDistance))) (.y _returnvalue) (.z _returnvalue)) false false))