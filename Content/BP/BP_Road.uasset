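; BP_Road builds a rolling road from chained BP_RoadSegment actors and registers itself with GM_Main.
; It starts from a child-actor segment and spawns each new one at the last segment's AttachPoint2.
; Rotate counts steps toward VictoryCount, updates GM_Main's Progress, and, once Count reaches BufferMax, removes the oldest segment and appends another.
; On reaching VictoryCount, it spawns BP_RoadFinalSegment at the end instead.
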(event EventBeginPlay
  (CallFunction|InitRoad)
  (bind _asgm_main (Utilities|Casting|CastToGM_Main (Game|GetGameMode)))
  (Variables|/Game/BP/GM_Main.GM_Main_C|SetRoad _asgm_main self))

(event EventActorBeginOverlap
  (params (OtherActor :type Actor%20Object%20Reference)))

(event EventTick
  (params (DeltaSeconds :type Float%20%28single-precision%29)))

(fn ConstructionScript)

(fn InitRoad
  (bind _asbp_road_segment (Utilities|Casting|CastToBP_RoadSegment (Variables|/Script/Engine.ChildActorComponent|GetChildActor (Variables|Default|GetStartSegment))))
  (Utilities|Array|Add (Variables|Default|GetRoadSegments) _asbp_road_segment)
  (for _index (range 0 (- (Variables|Default|GetInitialLength) 1))
    (CallFunction|AddNewSegment)))

(fn AddNewSegment
  (bind _roadsegments (Variables|Default|GetRoadSegments))
  (bind _returnvalue (Game|SpawnActorfromClass "/Game/BP/BP_RoadSegment.BP_RoadSegment_C" (Transformation|GetWorldTransform (Variables|/Game/BP/BP_RoadSegment.BP_RoadSegment_C|GetAttachPoint2 (Utilities|Array|Get(acopy) _roadsegments (Utilities|Array|LastIndex _roadsegments)))) "AlwaysSpawn" 0 0))
  (Utilities|Array|Add (Variables|Default|GetRoadSegments) _returnvalue)
  (Class|Actor|AttachRootComponentto _returnvalue (Variables|Default|GetDefaultSceneRoot) "None" "KeepWorldPosition" true))

(fn RemoveOldestSegment
  (bind _roadsegments (Variables|Default|GetRoadSegments))
  (bind _output_get (LocalVariables|Setdestroyed (Utilities|Array|Get(acopy) _roadsegments)))
  (Default|Clear _output_get)
  (Utilities|Array|RemoveItem _roadsegments _output_get)
  (Actor|DestroyActor _output_get))

(fn Rotate
  (if (not (== (Variables|Default|GetCount) (Variables|Default|GetVictoryCount)))
    (bind _output_get (Variables|Default|SetCount (+ (Variables|Default|GetCount) 1)))
    (bind _asgm_main (Utilities|Casting|CastToGM_Main (Game|GetGameMode)))
    (Variables|/Game/BP/GM_Main.GM_Main_C|SetProgress _asgm_main (/ (Math|Conversions|ToFloat(Integer) _output_get) (Math|Conversions|ToFloat(Integer) (Variables|Default|GetVictoryCount))))
    (if (>= _output_get (Variables|Default|GetBufferMax))
      (CallFunction|RemoveOldestSegment)
      (if (>= _output_get (Variables|Default|GetVictoryCount))
        (CallFunction|AttachFinalSegment)
        (else
          (CallFunction|AddNewSegment))))))

(fn AttachFinalSegment
  (bind _roadsegments (Variables|Default|GetRoadSegments))
  (Game|SpawnActorfromClass "/Game/BP/BP_RoadFinalSegment.BP_RoadFinalSegment_C" (Math|Transform|MakeTransform (Transformation|GetWorldLocation (Variables|/Game/BP/BP_RoadSegment.BP_RoadSegment_C|GetAttachPoint2 (Utilities|Array|Get(acopy) _roadsegments (Utilities|Array|LastIndex _roadsegments)))) "0, 0, 0" "1,1,1") "AlwaysSpawn" 0 0))