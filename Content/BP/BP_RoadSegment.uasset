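; A road segment for an endless skater runner that picks a random mesh and spawns random obstacles across three lanes on BeginPlay.
; Obstacles land at random X points within a lane's bounds and are tracked so Clear can destroy them.
; A rolled cat obstacle only sets a flag instead of spawning.
; On the skater's first entry, it rotates GM_Main's road, advances progress, and triggers the cat playground's SpawnCat if flagged.
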(event OnComponentBeginOverlap(PlayerEntryCollision)
  (params (OtherActor :type Actor%20Object%20Reference) (OtherComp :type Primitive%20Component%20Object%20Reference) (OtherBodyIndex :type Integer) (bFromSweep :type Boolean) (SweepResult :type Hit%20Result%20Structure%20%28by%20ref%29))
  (Utilities|Casting|CastToSkaterDefaultPawn OtherActor)
  (if (not (Variables|Default|GetPassed))
    (bind _asgm_main (Utilities|Casting|CastToGM_Main (Game|GetGameMode)))
    (Default|Rotate (Variables|/Game/BP/GM_Main.GM_Main_C|GetRoad _asgm_main))
    (bind _asgm_main_2 (Utilities|Casting|CastToGM_Main (Game|GetGameMode)))
    (Default|IncreaseProgress _asgm_main_2)
    (Variables|Default|SetPassed true)
    (if (Variables|Default|GetSpawningCat)
      (bind _asgm_main_3 (Utilities|Casting|CastToGM_Main (Game|GetGameMode)))
      (bind _catplayground (Default|GetCatPlayGround _asgm_main_3))
      (Default|SpawnCat _catplayground))))

(event EventBeginPlay
  (bind _meshes (Variables|Default|GetMeshes))
  (Components|StaticMesh|SetStaticMesh (Variables|Default|GetStaticMesh) (Utilities|Array|Get(acopy) _meshes (Math|Random|RandomInteger (Utilities|Array|Length _meshes))))
  (CallFunction|SpawnRandom (Variables|Default|GetNumberOfObstacles)))

(fn ConstructionScript)

(fn SpawnRandomElementatLane
  (params (Lane :type Static%20Mesh%20Component%20Object%20Reference) (Obstacle%20Type :type BP%20Obstacle%20Class%20Reference))
  (bind _returnvalue (Transformation|GetWorldTransform Lane))
  (bind (_origin _boxextent) (Collision|GetComponentBounds Lane))
  (bind _returnvalue_2 (Game|SpawnActorfromClass Obstacle%20Type (Math|Transform|MakeTransform (Math|Vector|MakeVector (.x (Math|Random|RandomPointinBoundingBox _origin _boxextent)) (.y (.location _returnvalue)) (.z (.location _returnvalue))) (.rotation _returnvalue) "1,1,1") "AlwaysSpawn" 0 0))
  (Utilities|Array|Add (Variables|Default|GetSpawns) _returnvalue_2))

(fn GetRandomObstacleClass
  (bind _obstacles (Variables|Default|GetObstacles))
  (return (Utilities|Array|Get(acopy) _obstacles (Math|Random|RandomInteger (Utilities|Array|Length _obstacles)))))

(fn SpawnRandom
  (params (Count :type Integer))
  (for _index (range 1 Count)
    (bind _class (CallFunction|GetRandomObstacleClass))
    (if (Utilities|IsValidClass _class)
      (if (== _class "/Game/BP/Obstacles/BP_Obstacle_Cat.BP_Obstacle_Cat_C")
        (Variables|Default|SetSpawningCat true)
        (else
          (switch int (Math|Random|RandomInteger 3)
            (:0
              (CallFunction|SpawnRandomElementatLane (Variables|Default|GetLeftLane) _class))
            (:1
              (CallFunction|SpawnRandomElementatLane (Variables|Default|GetMiddleLane) _class))
            (:2
              (CallFunction|SpawnRandomElementatLane (Variables|Default|GetRightLane) _class))))))))

(fn Clear
  (for _array_element (Variables|Default|GetSpawns)
    (if (Utilities|IsValid _array_element)
      (Actor|DestroyActor _array_element))))