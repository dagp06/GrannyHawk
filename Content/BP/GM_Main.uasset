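; Main game mode for a God-versus-Granny game, tracking match time, bad luck, gate progress and the winner.
; Tick awards God the win at DefeatTime and adds bad luck every second, capped at the tier 3 amount.
; Victory functions lock out the opposing result and flag the Player; Granny's win is triggered externally.
; Helpers pass UI object selection to God, fetch the cat playground and loop the misfortune eye-glow animation by timer.
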(event Custom|StartTimer
  (bind _returnvalue (Utilities|Time|SetTimerbyEvent (delegate Custom|EventSetNextFrame) 0.1 true))
  (Variables|Default|SetEndingHandle _returnvalue))

(event Custom|EventSetNextFrame
  (Default|SetNextEyeGlowFrame (Variables|Default|GetUI_Misfortune)))

(event EventTick
  (params (DeltaSeconds :type Float%20%28single-precision%29))
  (bind _output_get (Variables|Default|Settime (+ (Variables|Default|Gettime) DeltaSeconds)))
  (if (>= _output_get (Variables|Default|GetDefeatTime))
    (CallFunction|VictoryGod))
  (bind _output_get_2 (Variables|Default|Setsecondtimer (+ (Variables|Default|Getsecondtimer) DeltaSeconds)))
  (if (>= _output_get_2 1.0)
    (Variables|Default|Setsecondtimer 0.0)
    (CallFunction|AddBadluck 3.0)))

(fn ConstructionScript)

(fn GetCatPlayGround
  (bind _asbp_cat_playground (Utilities|Casting|CastToBP_CatPlayground (Variables|/Script/Engine.ChildActorComponent|GetChildActor (Variables|/Game/BP/BP_PlayZone.BP_PlayZone_C|GetBP_CatPlayground (Variables|Default|GetPlayZone)))))
  (return _asbp_cat_playground))

(fn AddBadluck
  (params (delta :type Float%20%28single-precision%29))
  (bind _tier3amount (Variables|Default|GetTier3Amount))
  (if (not (or (Variables|Default|GetGodWon) (Variables|Default|GetGrannyWon)))
    (bind _output_get (Variables|Default|SetBadluck (+ delta (Variables|Default|GetBadluck))))
    (if (>= _output_get _tier3amount)
      (Variables|Default|SetBadluck _tier3amount)
      (elif (<= _tier3amount 0.0)
        (Variables|Default|SetBadluck 0.0)))))

(fn SelectNextFallingObject
  (bind _objectnumber (Default|SelectNextObject (Variables|Default|GetUI_ObjectSelection)))
  (CallFunction|SetCurrentObject _objectnumber))

(fn SetCurrentObject
  (params (objectNumber :type Integer))
  (Default|SetCurrentObject (Variables|Default|GetGod) objectNumber))

(fn VictoryGranny
  (if (not (or (Variables|Default|GetGrannyWon) (Variables|Default|GetGodWon)))
    (Development|PrintString "Granny has won" true true "(R=0.124446,G=1.000000,B=0.000000,A=1.000000)" 2e+01)
    (bind _output_get (Variables|Default|SetGrannyWon true))
    (Variables|/Game/ThirdPersonBP/Blueprints/SkaterDefaultPawn.SkaterDefaultPawn_C|SetGrannyWins (Variables|Default|GetPlayer) _output_get)))

(fn VictoryGod
  (bind _player (Variables|Default|GetPlayer))
  (if (not (or (Variables|Default|GetGrannyWon) (Variables|Default|GetGodWon)))
    (bind _output_get (Variables|Default|SetGodWon true))
    (Variables|/Game/ThirdPersonBP/Blueprints/SkaterDefaultPawn.SkaterDefaultPawn_C|SetGodWins _player _output_get)
    (Default|StopGranny _player)))

(fn IncreaseProgress
  (bind _result (Math|Integer|IncrementInt (Variables|Default|GetGatePassed))
    (:%20%20
      (Variables|Default|SetProgress (/ (Math|Conversions|ToFloat(Integer) _result) (Math|Conversions|ToFloat(Integer) (Variables|Default|GetPathLength)))))))