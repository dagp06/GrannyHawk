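; BP_Obstacle_Cat is a moving cat obstacle that reacts when the skater runs into it.
; It activates CatAppear on BeginPlay, then moves along its forward vector at Speed each tick without sweeping.
; A skeletal mesh overlap with a SkaterDefaultPawn plays the hit sound cue.
; Tick destroys the actor once Lifetime reaches zero, but the subtraction is zero, so Lifetime never counts down here.
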(event OnComponentBeginOverlap(SkeletalMesh)
  (params (OtherActor :type Actor%20Object%20Reference) (OtherComp :type Primitive%20Component%20Object%20Reference) (OtherBodyIndex :type Integer) (bFromSweep :type Boolean) (SweepResult :type Hit%20Result%20Structure%20%28by%20ref%29))
  (if (Utilities|ClassIsChildOf (Utilities|GetClass OtherActor) "/Game/ThirdPersonBP/Blueprints/SkaterDefaultPawn.SkaterDefaultPawn_C")
    (Audio|Components|Audio|Play (Variables|Default|GetCat_Hit_new_Cue) 0.0)))

(event EventBeginPlay
  (Components|Activation|Activate (Variables|Default|GetCat_Appear) false))

(event EventTick
  (params (DeltaSeconds :type Float%20%28single-precision%29))
  (Transformation|AddActorWorldOffset (* (* (Transformation|GetActorForwardVector) DeltaSeconds) (Variables|Default|GetSpeed)))
  (bind _output_get (Variables|Default|SetLifetime (- (Variables|Default|GetLifetime) 0.0)))
  (if (<= _output_get 0.0)
    (Actor|DestroyActor)))

(fn ConstructionScript
  (|CallParentFunction))