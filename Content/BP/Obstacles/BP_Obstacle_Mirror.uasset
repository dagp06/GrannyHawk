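; Breakable mirror obstacle that shatters when the skater pawn runs into it.
; On collision box overlap by a SkaterDefaultPawn, it applies full radius damage at the destructible mesh's origin, activates the hit cue and prints a debug string.
; The box's collision is then disabled so the hit is not repeated.
; An alternative directional ApplyDamage impulse is left unconnected.
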(event OnComponentBeginOverlap(CollisionBox)
  (params (OtherActor :type Actor%20Object%20Reference) (OtherComp :type Primitive%20Component%20Object%20Reference) (OtherBodyIndex :type Integer) (bFromSweep :type Boolean) (SweepResult :type Hit%20Result%20Structure%20%28by%20ref%29))
  (if (Utilities|ClassIsChildOf (Utilities|GetClass OtherActor) "/Game/ThirdPersonBP/Blueprints/SkaterDefaultPawn.SkaterDefaultPawn_C")
    (Class|DestructibleComponent|ApplyRadiusDamage (Variables|Default|GetSM_Mirror_DM) 1e+03 (Transformation|GetWorldLocation (Variables|Default|GetSM_Mirror_DM)) 0.0 0.0 true)
    (Development|PrintString "BP_OBSTACLE_MIRROR")
    (Components|Activation|Activate (Variables|Default|GetEnv_Miroir_Hit_Cue) true)
    (Collision|SetCollisionEnabled (Variables|Default|GetCollisionBox) "NoCollision")))

(event EventBeginPlay)

(event EventActorBeginOverlap
  (params (OtherActor :type Actor%20Object%20Reference)))

(event EventTick
  (params (DeltaSeconds :type Float%20%28single-precision%29)))

(fn ConstructionScript
  (|CallParentFunction))